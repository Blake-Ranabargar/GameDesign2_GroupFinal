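; BP_NaginataPedestal is a pedestal where the player returns a held naginata as part of a weapon-return objective.
; Entering its box trigger as the third-person character shows a hint widget, created at BeginPlay, which is removed when an overlap ends.
; If BP_Gamemanager reports the naginata as held, the overlap increments its returned-weapon count, clears the held flag, reveals the pedestal's naginata mesh and runs the manager's elevator check.
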(event OnComponentBeginOverlap(Box)
  (params (OverlappedComponent :type Primitive%20Component%20Object%20Reference) (OtherActor :type Actor%20Object%20Reference) (OtherComp :type Primitive%20Component%20Object%20Reference) (OtherBodyIndex :type Integer) (bFromSweep :type Boolean) (SweepResult :type Hit%20Result%20Structure%20%28by%20ref%29))
  (Utilities|Casting|CastToBP_ThirdPersonCharacter OtherActor)
  (UserInterface|Viewport|AddtoViewport (Variables|Default|GetW_NaginataHint) 0)
  (bind _returnvalue (Actor|GetActorOfClass "/Game/Dev_Folders/Orin/Blueprints/BP_Gamemanager.BP_Gamemanager_C"))
  (if (Variables|/Game/Dev_Folders/Orin/Blueprints/BP_Gamemanager.BP_Gamemanager_C|GetNaginataHeld _returnvalue)
    (bind _result (Math|Integer|IncrementInt (Variables|/Game/Dev_Folders/Orin/Blueprints/BP_Gamemanager.BP_Gamemanager_C|GetWeaponsReturned _returnvalue))
      (:%20%20
        (Variables|/Game/Dev_Folders/Orin/Blueprints/BP_Gamemanager.BP_Gamemanager_C|SetWeaponsReturned _returnvalue _result)
        (Variables|/Game/Dev_Folders/Orin/Blueprints/BP_Gamemanager.BP_Gamemanager_C|SetNaginataHeld _returnvalue false)
        (Development|SetHiddeninGame (Variables|Default|GetSM_Wep_Naginata_02) false false)
        (Default|ElevatorCheck _returnvalue)))))

(event OnComponentEndOverlap(Box)
  (params (OverlappedComponent :type Primitive%20Component%20Object%20Reference) (OtherActor :type Actor%20Object%20Reference) (OtherComp :type Primitive%20Component%20Object%20Reference) (OtherBodyIndex :type Integer))
  (Widget|RemovefromParent (Variables|Default|GetW_NaginataHint)))

(event EventBeginPlay
  (bind _returnvalue (UserInterface|CreateWidget "/Game/Dev_Folders/Orin/Blueprints/W_NaginataHint.W_NaginataHint_C"))
  (Variables|Default|SetW_NaginataHint _returnvalue))

(fn ConstructionScript)
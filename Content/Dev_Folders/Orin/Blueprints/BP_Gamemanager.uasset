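; BP_Gamemanager controls when the level's enter and leave elevators are visible, based on returned weapons.
; On BeginPlay it hides BP_Elevator_Leave_Blake, then hides BP_Elevator_Enter after a short delay.
; ElevatorCheck unhides the leave elevator once WeaponsReturned reaches the required count; nothing in this graph changes that count or calls the check.
; Elevators are found by class lookup, and only their hidden-in-game state changes.
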(event Custom|ElevatorCheck
  (if (== (Variables|Default|GetWeaponsReturned) 3)
    (bind _returnvalue (Actor|GetActorOfClass "/Game/Dev_Folders/Blake/BPs/BP_Elevator_Leave_Blake.BP_Elevator_Leave_Blake_C"))
    (Rendering|SetActorHiddenInGame _returnvalue false)))

(event EventBeginPlay
  (bind _returnvalue (Actor|GetActorOfClass "/Game/Dev_Folders/Blake/BPs/BP_Elevator_Leave_Blake.BP_Elevator_Leave_Blake_C"))
  (Rendering|SetActorHiddenInGame _returnvalue true)
  (Utilities|FlowControl|Delay 1e+01)
  (bind _returnvalue_2 (Actor|GetActorOfClass "/Game/Dev_Folders/Blake/BPs/BP_Elevator_Enter.BP_Elevator_Enter_C"))
  (Rendering|SetActorHiddenInGame _returnvalue_2 true))

(fn ConstructionScript)
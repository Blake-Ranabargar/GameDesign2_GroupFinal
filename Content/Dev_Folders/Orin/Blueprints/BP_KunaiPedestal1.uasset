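; BP_KunaiPedestal1 is a pedestal where the player returns a found kunai weapon.
; When the third-person character enters its box trigger, it checks KunaiHeld on BP_Gamemanager.
; If held, it increments WeaponsReturned, clears the flag, unhides the kunai mesh and calls the manager's ElevatorCheck.
; Otherwise it prints that the weapon has not been found yet.
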(event OnComponentBeginOverlap(Box)
  (params (OverlappedComponent :type Primitive%20Component%20Object%20Reference) (OtherActor :type Actor%20Object%20Reference) (OtherComp :type Primitive%20Component%20Object%20Reference) (OtherBodyIndex :type Integer) (bFromSweep :type Boolean) (SweepResult :type Hit%20Result%20Structure%20%28by%20ref%29))
  (Utilities|Casting|CastToBP_ThirdPersonCharacter OtherActor)
  (bind _returnvalue (Actor|GetActorOfClass "/Game/Dev_Folders/Orin/Blueprints/BP_Gamemanager.BP_Gamemanager_C"))
  (if (Variables|/Game/Dev_Folders/Orin/Blueprints/BP_Gamemanager.BP_Gamemanager_C|GetKunaiHeld _returnvalue)
    (bind _result (Math|Integer|IncrementInt (Variables|/Game/Dev_Folders/Orin/Blueprints/BP_Gamemanager.BP_Gamemanager_C|GetWeaponsReturned _returnvalue))
      (:%20%20
        (Variables|/Game/Dev_Folders/Orin/Blueprints/BP_Gamemanager.BP_Gamemanager_C|SetWeaponsReturned _returnvalue _result)
        (Variables|/Game/Dev_Folders/Orin/Blueprints/BP_Gamemanager.BP_Gamemanager_C|SetKunaiHeld _returnvalue false)
        (Development|SetHiddeninGame (Variables|Default|GetSM_Wep_Kunai_01) false false)
        (Default|ElevatorCheck _returnvalue)))
    (else
      (Development|PrintString "You have yet to find this weapon"))))

(fn ConstructionScript)
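; BP_NPC is a talking NPC that loops an idle animation and shows dialogue to the player.
; Capsule overlap plays a half-speed talking montage, returning to idle on blend out.
; Sphere overlap registers the NPC on BP_ThirdPersonCharacter, shows WTalk and calls NextLine to step through Dialogue.
; The widget is created only after that step, and creation and a sound run for any overlapping actor.
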(event OnComponentBeginOverlap(Capsule)
  (params (OverlappedComponent :type Primitive%20Component%20Object%20Reference) (OtherActor :type Actor%20Object%20Reference) (OtherComp :type Primitive%20Component%20Object%20Reference) (OtherBodyIndex :type Integer) (bFromSweep :type Boolean) (SweepResult :type Hit%20Result%20Structure%20%28by%20ref%29))
  ;[0.15 0.15 0.15 0.5] NPC - Talk to player & play animation
  (Utilities|FlowControl|Sequence
    (:then_0
      (Animation|Montage|PlayMontage (Variables|Default|GetSkeletalMesh) "/Game/Talking_Anim_Montage.Talking_Anim_Montage" 0.5
        (:OnBlendOut
          (Components|Animation|PlayAnimation (Variables|Default|GetSkeletalMesh) "/Game/MM_Idle_MontageSYNTY.MM_Idle_MontageSYNTY" true))))))

(event OnComponentBeginOverlap(Sphere)
  (params (OverlappedComponent :type Primitive%20Component%20Object%20Reference) (OtherActor :type Actor%20Object%20Reference) (OtherComp :type Primitive%20Component%20Object%20Reference) (OtherBodyIndex :type Integer) (bFromSweep :type Boolean) (SweepResult :type Hit%20Result%20Structure%20%28by%20ref%29))
  (Utilities|FlowControl|Sequence
    (:then_0
      (bind _asbp_third_person_character (Utilities|Casting|CastToBP_ThirdPersonCharacter OtherActor))
      (bind _output_get (Variables|Default|SetPlayer _asbp_third_person_character))
      (Variables|/Game/ThirdPerson/Blueprints/BP_ThirdPersonCharacter.BP_ThirdPersonCharacter_C|SetNPC _output_get self)
      (UserInterface|Viewport|AddtoViewport (Variables|Default|GetW_Talk) 0)
      (CallFunction|NextLine))
    (:then_1
      (bind _returnvalue (UserInterface|CreateWidget "/Game/Dev_Folders/JP/Widgets/W_TalkWidget.W_TalkWidget_C"))
      (Variables|Default|SetW_Talk _returnvalue))
    (:then_2
      ;[0.15 0.15 0.15 0.5] NPC - Talk to player & play animation
      (Audio|PlaySound2D "/Game/LieDown.LieDown" 1.0 1.0 0.0 0 0))))

(event Custom|Next%20Line
  (Rendering|Components|TextRender|SetText (Variables|/Game/Dev_Folders/JP/Widgets/W_TalkWidget.W_TalkWidget_C|GetTextBlock_0 (Variables|Default|GetW_Talk)) (Utilities|Array|Get(acopy) (Variables|Default|GetDialogue) (Variables|Default|GetLineIndex)))
  (Math|Integer|IncrementInt (Variables|Default|GetLineIndex)))

(event EventBeginPlay
  ;[0.15 0.15 0.15 0.5] NPC - Talk to player & play animation
  (Utilities|FlowControl|Sequence
    (:then_0
      (Components|Animation|PlayAnimation (Variables|Default|GetSkeletalMesh) "/Game/MM_Idle_MontageSYNTY.MM_Idle_MontageSYNTY" true))))

(fn ConstructionScript)
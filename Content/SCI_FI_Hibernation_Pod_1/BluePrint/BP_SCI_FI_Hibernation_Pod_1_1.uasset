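; Hibernation pod actor that acts as a level transition when the third-person character enters its trigger box.
; On overlap it snaps the pod mesh to a fixed rotation, plays a quick-breath sound at world origin, then opens the level in LevelName after a short delay.
; A separate OpenDoor event uses a timeline to raise the mesh along Z, but nothing in this graph calls it.
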(event OnComponentBeginOverlap(Box)
  (params (OverlappedComponent :type Primitive%20Component%20Object%20Reference) (OtherActor :type Actor%20Object%20Reference) (OtherComp :type Primitive%20Component%20Object%20Reference) (OtherBodyIndex :type Integer) (bFromSweep :type Boolean) (SweepResult :type Hit%20Result%20Structure%20%28by%20ref%29))
  (Utilities|Casting|CastToBP_ThirdPersonCharacter OtherActor)
  (Transformation|SetRelativeRotation (Variables|Default|GetSM_SCI_FI_Hibernation_Pod_1_Asset_1) "59.000000,110.000000,107.000000" false false)
  (Utilities|FlowControl|Sequence
    (:then_0
      (Audio|PlaySoundatLocation "/Game/Dev_Folders/Blake/Sounds/SW_QuickBreath.SW_QuickBreath" "0, 0, 0" "0, 0, 0" 1.0 1.0 0.0 0 0 0 0))
    (:then_1
      (Utilities|FlowControl|Delay 4.0)
      (Game|OpenLevel(byName) (Variables|Default|GetLevel%20Name)))))

(event Custom|Open%20Door
  (bind _door_float (Timeline|Door%20TL Play)
    (:Update
      (Transformation|SetRelativeLocationAndRotation (Variables|Default|GetSM_SCI_FI_Hibernation_Pod_1_Asset_1) (Math|Vector|Lerp(Vector) "0, 0, 0" "0.000000,0.000000,290.000000" _door_float) "0, 0, 0" false false))))

(fn ConstructionScript)